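; BP_Tunnel is a tunnel segment with a rotating holed wall for an endless dodge game.
; Tick spins the wall, and RandomizeWall, not called here, picks one of four hole meshes.
; When BP_Player enters the box, the segment requests a new tunnel spawn and destroys itself, with end overlap incrementing score.
; Hitting the wall marks the player dead, stops rotation and shows the restart display with the score.
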(event OnComponentBeginOverlap(Box)
  (params (OverlappedComponent :type Primitive%20Component%20Object%20Reference) (OtherActor :type Actor%20Object%20Reference) (OtherComp :type Primitive%20Component%20Object%20Reference) (OtherBodyIndex :type Integer) (bFromSweep :type Boolean) (SweepResult :type Hit%20Result%20Structure%20%28by%20ref%29))
  (Utilities|Casting|CastToBP_Player OtherActor)
  (Default|SpawnTunnelatSpawnPoint (Variables|Default|GetReference))
  (Actor|DestroyActor))

(event OnComponentHit(WallMesh)
  (params (HitComponent :type Primitive%20Component%20Object%20Reference) (OtherActor :type Actor%20Object%20Reference) (OtherComp :type Primitive%20Component%20Object%20Reference) (NormalImpulse :type Vector :default "0, 0, 0") (Hit :type Hit%20Result%20Structure%20%28by%20ref%29))
  ;[1 1 1] Dead
  (bind _asbp_player (Utilities|Casting|CastToBP_Player OtherActor))
  (Variables|/Game/InfiniteMatrix/Blueprints/BP_Player.BP_Player_C|SetDead _asbp_player true)
  (Variables|Default|SetRotateSpeed 0)
  (Default|DisplayReastart _asbp_player (Variables|/Game/InfiniteMatrix/Blueprints/BP_Player.BP_Player_C|GetScore _asbp_player)))

(event OnComponentEndOverlap(Box)
  (params (OverlappedComponent :type Primitive%20Component%20Object%20Reference) (OtherActor :type Actor%20Object%20Reference) (OtherComp :type Primitive%20Component%20Object%20Reference) (OtherBodyIndex :type Integer))
  ;[1 1 1] Score
  (bind _asbp_player (Utilities|Casting|CastToBP_Player OtherActor))
  (Math|Integer|IncrementInt (Variables|/Game/InfiniteMatrix/Blueprints/BP_Player.BP_Player_C|GetScore _asbp_player)))

(event EventBeginPlay)

(event EventTick
  (params (DeltaSeconds :type Float%20%28single-precision%29))
  ;[1 1 1] Rotate Wall
  (Transformation|AddLocalRotation (Variables|Default|GetWallMesh) (Math|Rotator|MakeRotator (* (Variables|Default|GetRotateSpeed) DeltaSeconds) 0.0 0.0) false false))

(fn ConstructionScript)

(fn RandomizeWall
  (Components|StaticMesh|SetStaticMesh (Variables|Default|GetWallMesh) (Utilities|Select :Index (Math|Random|RandomIntegerinRange 0 3) :Option%200 "/Game/InfiniteMatrix/Meshes/SM_Hole_01.SM_Hole_01" :Option%201 "/Game/InfiniteMatrix/Meshes/SM_Hole_02.SM_Hole_02" :Option%202 "/Game/InfiniteMatrix/Meshes/SM_Hole_03.SM_Hole_03" :Option%203 "/Game/InfiniteMatrix/Meshes/SM_Hole_04.SM_Hole_04")))